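; Spawn marker actor for Deathmatch and Gun Game modes in a custom map.
; On BeginPlay the server checks whether the game mode's display name starts with DeathMatch, GunGame or WW2GunGame, and destroys the actor in any other mode.
; The construction script applies the TeamColor material to the DMGGSpawn component.
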(event `self.ReceiveBeginPlay`
  (`/Engine/EditorBlueprintResources/ActorMacros.Switch Has Authority`
    (:`Authority`
      (if (not (or (`KismetStringLibrary.StartsWith` (`KismetSystemLibrary.GetDisplayName` (`GameplayStatics.GetGameMode`)) "DeathMatch" "CaseSensitive") (`KismetStringLibrary.StartsWith` (`KismetSystemLibrary.GetDisplayName` (`GameplayStatics.GetGameMode`)) "GunGame" "CaseSensitive") (`KismetStringLibrary.StartsWith` (`KismetSystemLibrary.GetDisplayName` (`GameplayStatics.GetGameMode`)) "WW2GunGame" "CaseSensitive")))
        (`self.K2_DestroyActor`)))))

(fn `UserConstructionScript`
  (`PrimitiveComponent.SetMaterial` (`self.DM_GG_Spawn`) 0 (`self.TeamColor`)))